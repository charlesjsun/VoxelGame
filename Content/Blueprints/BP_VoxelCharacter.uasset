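; Voxel-building character that previews the targeted face and where the selected voxel would go.
; BeginPlay spawns a BP_VoxelOutline actor; each Tick, with valid terrain and a VoxelPlayerController, it ray-traces voxel coordinates within reach.
; On a hit, the face marker aligns to the hit normal, and a ghost tinted with the selected voxel type's color moves to the adjacent cell.
; Both hide on a miss; only the ghost hides when no voxel is selected.
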(event EventBeginPlay
  (bind _returnvalue (Game|SpawnActorfromClass "/Game/Blueprints/BP_VoxelOutline.BP_VoxelOutline_C" (Math|Transform|MakeTransform "0, 0, 0") "AlwaysSpawn" self 0))
  (Variables|Default|SetVoxelOutline _returnvalue))

(event EventTick
  (params (DeltaSeconds :type Float%20%28single-precision%29))
  (bind _returnvalue (Pawn|GetController))
  (bind _voxeloutline (Variables|Default|GetVoxelOutline))
  (bind _voxeloutline_2 (Variables|Default|GetVoxelOutline))
  (bind _voxeloutline_3 (Variables|Default|GetVoxelOutline))
  (bind (_asvoxel_player_controller _bsuccess) (Utilities|Casting|CastToVoxelPlayerController _returnvalue))
  (bind _voxelface (Variables|/Game/Blueprints/BP_VoxelOutline.BP_VoxelOutline_C|GetVoxelFace _voxeloutline_3))
  (if (and (Utilities|IsValid (Variables|Default|GetVoxelTerrain)) _bsuccess)
    (bind (_outvoxelcoord _outhitnormal _returnvalue_2) (Class|VoxelPlayerController|RayTraceVoxelCoord _asvoxel_player_controller (Variables|Default|GetReachDistance)))
    (if _returnvalue_2
      (Rendering|SetVisibility (Variables|/Game/Blueprints/BP_VoxelOutline.BP_VoxelOutline_C|GetVoxelGhost _voxeloutline_3) true false)
      (Rendering|SetVisibility _voxelface true false)
      (Transformation|SetWorldLocationAndRotation _voxelface (+ (* (Class|VoxelMathLibrary|ToVector(IntVector3) _outhitnormal) -5e+01) (* (+ (+ (Class|VoxelMathLibrary|ToVector(IntVector3) _outhitnormal) (Class|VoxelMathLibrary|ToVector(IntVector3) _outvoxelcoord)) 0.5) 1e+02)) (Math|Rotator|MakeRotfromZ (Class|VoxelMathLibrary|ToVector(IntVector3) _outhitnormal)) false true)
      (if (== (Variables|Default|GetCurrentVoxel) 0)
        ;[1 1 1] If no voxel is selected
        (Rendering|SetVisibility (Variables|/Game/Blueprints/BP_VoxelOutline.BP_VoxelOutline_C|GetVoxelGhost _voxeloutline) false false :!label _label)
        (else
          (Transformation|SetActorLocation _voxeloutline_2 (* (+ (+ (Class|VoxelMathLibrary|ToVector(IntVector3) _outhitnormal) (Class|VoxelMathLibrary|ToVector(IntVector3) _outvoxelcoord)) 0.5) 1e+02) false false)
          (Rendering|Material|SetVectorParameterValueonMaterials (Variables|/Game/Blueprints/BP_VoxelOutline.BP_VoxelOutline_C|GetVoxelGhost _voxeloutline_2) "VoxelColor" (Math|Conversions|ToVector(LinearColor) (Math|Conversions|ToLinearColor(Color) (.VoxelColor (Utilities|Struct|BreakVoxelType (Class|VoxelTerrain|GetVoxelType (Variables|Default|GetVoxelTerrain) (Math|Conversions|ToByte(Integer) (Variables|Default|GetCurrentVoxel))))))))))
      (else
        (Rendering|SetVisibility (Variables|/Game/Blueprints/BP_VoxelOutline.BP_VoxelOutline_C|GetVoxelFace _voxeloutline) false false)
        (goto _label)))))

(fn ConstructionScript)